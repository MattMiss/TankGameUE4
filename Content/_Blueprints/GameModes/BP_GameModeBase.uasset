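; Base game mode Blueprint that runs a wave-based enemy game's start, round transition and game-over events.
; It shows the matching widget for each event, with sounds at start and end, and teleports the player to spawn between rounds.
; SpawnNextWave builds enemies from WaveEnemySpawner data, passing roam and patrol settings to cannons.
; Spawned enemies are tracked in EnemiesInWave, which UnfreezeEnemies uses to release them.
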(event Custom|MovePlayerToStart
  ;[1 1 1] Transport Player to Start
  (Utilities|FlowControl|Delay 1.0)
  (Transformation|SetActorLocationAndRotation (Game|Player|GetPlayerPawn 0) (Variables|Default|GetSpawnLocation) (Variables|Default|GetSpawnRotation) false true))

(event Custom|UnfreezeEnemies
  (for _array_element (Variables|Default|GetEnemiesInWave)
    (bind _aspawn_turret (Utilities|Casting|CastToPawnTurret _array_element))
    (Class|PawnTurret|UnfreezeatStart _aspawn_turret)))

(event EventSpawnNextWave
  (params (WaveIndex :type Integer))
  (bind _returnvalue (+ WaveIndex 1))
  (bind _waveenemyspawner (Variables|Default|GetWaveEnemySpawner))
  (bind _wavespawninfo (Variables|/Script/ToonTanks.WaveEnemySpawner|GetWaveSpawnInfo _waveenemyspawner))
  ;[1 1 1] Spawn the Next Wave
  (if (<= _returnvalue (Utilities|Array|Length _wavespawninfo))
    (for _array_element (Utilities|Struct|BreakWaveSpawnInfo (Utilities|Array|Get(acopy) _wavespawninfo WaveIndex))
      (bind _returnvalue_2 (Game|SpawnActorfromClass (.EnemyClass (Utilities|Struct|BreakEnemySpawnInfo _array_element)) (Math|Transform|MakeTransform (.SpawnLocation (Utilities|Struct|BreakEnemySpawnInfo _array_element)) (.SpawnRotation (Utilities|Struct|BreakEnemySpawnInfo _array_element))) "AdjustIfPossibleButAlwaysSpawn" 0 0))
      (Utilities|Array|Add (Variables|Default|GetEnemiesInWave) _returnvalue_2)
      (if (Utilities|Enum|Equal(Enum) (.EnemyType (Utilities|Struct|BreakEnemySpawnInfo _array_element)) "Turret")
        (Utilities|Casting|CastToBP_PawnTurret _returnvalue_2)
        (elif (Utilities|Enum|Equal(Enum) (.EnemyType (Utilities|Struct|BreakEnemySpawnInfo _array_element)) "Cannon")
          (bind _asbp_pawn_cannon (Utilities|Casting|CastToBP_PawnCannon _returnvalue_2))
          (Variables|/Script/ToonTanks.PawnTurret|SetCanRoam _asbp_pawn_cannon (.CanRoam (Utilities|Struct|BreakEnemySpawnInfo _array_element)))
          (Variables|/Script/ToonTanks.PawnTurret|SetPatrolPoints _asbp_pawn_cannon (.PatrolPoints (Utilities|Struct|BreakEnemySpawnInfo _array_element))))))
    (else
      (Development|PrintString (Utilities|String|Append "WaveSpawner does not contain a wave  " (Utilities|String|ToString(Integer) _returnvalue))))))

(event EventNextRound
  (params (RoundNum :type Integer))
  ;[1 1 1] Next Round
  (bind _returnvalue (UserInterface|CreateWidget "/Game/_Blueprints/Widgets/WBP_NextRound.WBP_NextRound_C"))
  (Variables|/Game/_Blueprints/Widgets/WBP_NextRound.WBP_NextRound_C|SetRoundNumber _returnvalue (+ RoundNum 1))
  (Default|SetStartDelay _returnvalue 4)
  (UserInterface|Viewport|AddtoViewport _returnvalue 0)
  (CallFunction|MovePlayertoStart))

(event EventGameStart
  ;[1 1 1] Game Start
  (bind _returnvalue (UserInterface|CreateWidget "/Game/_Blueprints/Widgets/WBP_GameStart.WBP_GameStart_C"))
  (Default|SetStartDelay _returnvalue 4)
  (UserInterface|Viewport|AddtoViewport _returnvalue 0)
  (Audio|PlaySound2D "/Game/Assets/Audio/Win_sound_1_Cue.Win_sound_1_Cue" 1.0 1.0 0.0 0 0))

(event EventGameOver
  (params (PlayerWon :type Boolean))
  (bind _returnvalue (Game|GetPlayerController 0))
  ;[1 1 1] Game Over
  (bind _returnvalue_2 (UserInterface|CreateWidget "/Game/_Blueprints/Widgets/WBP_GameEnd.WBP_GameEnd_C"))
  (Default|SetPlayerWon _returnvalue_2 PlayerWon)
  (UserInterface|Viewport|AddtoViewport _returnvalue_2 0)
  (Input|SetInputModeUIOnly _returnvalue _returnvalue_2 "DoNotLock")
  (Variables|/Script/Engine.PlayerController|SetbShowMouseCursor _returnvalue true)
  (Audio|PlaySound2D "/Game/Assets/Audio/Lose_sound_14_Cue.Lose_sound_14_Cue" 1.0 1.0 0.0 0 0))

(fn ConstructionScript)