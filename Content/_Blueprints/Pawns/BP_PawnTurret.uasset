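; BP_PawnTurret is a turret pawn that lobs bomb projectiles at the player.
; On FireBP, it spawns a hidden target decal just below the player's position and computes an arcing launch velocity from the projectile spawn point to the player.
; It then spawns the projectile, passes it the decal reference if it is a BP_ProjectileBomb, and overrides its movement velocity with the computed arc.
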(event EventFireBP
  (bind _returnvalue (Game|Player|GetPlayerPawn 0))
  (bind _self self)
  (bind _returnvalue_2 (Transformation|GetActorLocation _returnvalue))
  (bind (_x _y _z) (Math|Vector|BreakVector _returnvalue_2))
  (bind _returnvalue_3 (Game|SpawnActorfromClass "/Game/_Blueprints/Decals/BombDecal.BombDecal_C" (Math|Conversions|ToTransform(Vector) (Math|Vector|MakeVector _x _y (- _z 55.0))) "Undefined" 0 0))
  (bind _output_get (Variables|Default|SetCurrentTargetDecal _returnvalue_3))
  (Rendering|SetVisibility (Variables|/Script/Engine.DecalActor|GetDecal _output_get) false false)
  (bind _outlaunchvelocity (Game|SuggestProjectileVelocityCustomArc (Transformation|GetWorldLocation (Variables|Default|GetProjectileSpawnPoint)) _returnvalue_2 0.0 0.5))
  (bind _returnvalue_4 (Game|SpawnActorfromClass (Variables|Default|GetProjectileClass) (Transformation|GetWorldTransform (Variables|Default|GetProjectileSpawnPoint)) "Undefined" _self _self))
  (bind _asbp_projectile_bomb (Utilities|Casting|CastToBP_ProjectileBomb _returnvalue_4))
  (Variables|/Script/ToonTanks.ProjectileBase|SetHitDecalRef _asbp_projectile_bomb (Variables|Default|GetCurrentTargetDecal))
  (Variables|/Script/Engine.MovementComponent|SetVelocity (Variables|/Script/ToonTanks.ProjectileBase|GetProjectileMovement _asbp_projectile_bomb) _outlaunchvelocity))

(fn ConstructionScript)