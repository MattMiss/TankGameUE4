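; BP_PawnCannon is a cannon pawn that lobs arcing projectiles at the first player's current location.
; FireBP spawns a decal at that location as a hit marker, then spawns the projectile at the spawn point with the cannon as owner and instigator.
; It hands the decal to the BP_ProjectileBase projectile and sets its velocity from SuggestProjectileVelocityCustomArc.
; BeginPlay only prints the CanRoam value.
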(event EventBeginPlay
  (Development|PrintString (Utilities|String|ToString(Boolean) (Variables|Default|GetCanRoam))))

(event EventFireBP
  (bind _returnvalue (Game|Player|GetPlayerPawn 0))
  (bind _self self)
  (bind _returnvalue_2 (Transformation|GetActorLocation _returnvalue))
  (bind _returnvalue_3 (Game|SpawnActorfromClass "/Game/_Blueprints/Decals/CannonDecal.CannonDecal_C" (Math|Conversions|ToTransform(Vector) _returnvalue_2) "Undefined" 0 0))
  (Variables|Default|SetCurrentTargetDecal _returnvalue_3)
  (bind _outlaunchvelocity (Game|SuggestProjectileVelocityCustomArc (Transformation|GetWorldLocation (Variables|Default|GetProjectileSpawnPoint)) _returnvalue_2 0.0 0.5))
  (bind _returnvalue_4 (Game|SpawnActorfromClass (Variables|Default|GetProjectileClass) (Transformation|GetWorldTransform (Variables|Default|GetProjectileSpawnPoint)) "Undefined" _self _self))
  (bind _asbp_projectile_base (Utilities|Casting|CastToBP_ProjectileBase _returnvalue_4))
  (Variables|/Game/_Blueprints/Actors/BP_ProjectileBase.BP_ProjectileBase_C|SetHitDecalRef _asbp_projectile_base (Variables|Default|GetCurrentTargetDecal))
  (Variables|/Script/Engine.MovementComponent|SetVelocity (Variables|/Script/ToonTanks.ProjectileBase|GetProjectileMovement _returnvalue_4) _outlaunchvelocity))

(fn ConstructionScript)