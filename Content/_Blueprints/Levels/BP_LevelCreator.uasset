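; Level creator that shapes a grid of floor hexagons from the current level's data table, picked from a composite table's parent tables.
; It walks each row column by column through re-entrant event calls, pausing briefly between rows.
; Each cell byte lowers or raises its hexagon or marks a raised spawn, registering with the game mode, which is notified on completion.
; ChangeLevel steps between levels, freezing the tank and rebuilding the floor.
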(event Custom|SetHexagonHeight
  (bind _curhexrowindex (Variables|Default|GetCurHexRowIndex))
  ;[1 1 1] Setup Hexagons
  (Development|PrintString (Utilities|String|Append "Row Index " (Utilities|String|ToString(Integer) _curhexrowindex)))
  (CallFunction|GetDataTable _curhexrowindex))

(event Custom|GetDataTable
  (params (Index :type Integer))
  ;[1 1 1] Get Data Table for Each row
  (bind _returnvalue (Utilities|GetDataTableRow (Variables|Default|GetCurrentDataTableRef) (Utilities|String|StringToName (Utilities|String|ToString(Integer) Index)))
    (:then
      (if (not (< (Variables|Default|GetCurHexColIndex) (Variables|Default|GetAmountOfCols)))
        (bind _finished (CallFunction|ChangetoNextRow))
        (if _finished
          (Utilities|FlowControl|Delay 0.05)
          (CallFunction|SetHexagonHeight)
          (else
            (Variables|Default|SetCurHexRowIndex 0)
            (CallFunction|TellGameModetoStart)))
        (else
          (CallFunction|MoveNextColumn _returnvalue))))))

(event Custom|MoveHexagon
  (params (Hexagon :type BP%20Floor%20Hexagon%20Object%20Reference) (HeightByte :type Byte) (HexNum :type Integer))
  (bind _returnvalue (== HeightByte 2))
  (bind _returnvalue_2 (== HeightByte 1))
  (bind _gamemoderef (Variables|Default|GetGameModeRef))
  ;[1 1 1] Move Hexagon Based on Byte (0 = Lower, 1 = Raise)
  (Utilities|IsValid Hexagon
    (:Is%20Valid
      (if _returnvalue_2
        (Default|AddtoRaisedFloors _gamemoderef Hexagon :!label _label)
        (elif _returnvalue
          (Default|SetSpawnHexagon _gamemoderef Hexagon)
          (goto _label)
          (else
            _)))
      (Default|StartMoving Hexagon (or _returnvalue_2 _returnvalue) HexNum))
    (:Is%20Not%20Valid
      (Development|PrintString "Invalid Hexagon"))))

(event Custom|TellGameModeToStart
  ;[1 1 1] Tell Game Mode To Start
  (Default|LevelSetupFinished (Variables|Default|GetGameModeRef)))

(event Custom|ChangeLevel
  (params (GoToNextLevel :type Boolean))
  (bind _gamemoderef (Variables|Default|GetGameModeRef))
  ;[1 1 1] Change Level (True input = Next Level) or (False input = Previous Level)
  (if GoToNextLevel
    (bind _datatableref (CallFunction|LoadNextLevel))
    (bind _output_get (Variables|Default|SetCurrentDataTableRef _datatableref))
    (Development|PrintString (Utilities|GetDisplayName _output_get))
    (else
      (bind _datatableref_2 (CallFunction|LoadPreviousLevel))
      (bind _output_get_2 (Variables|Default|SetCurrentDataTableRef _datatableref_2))
      (Development|PrintString (Utilities|GetDisplayName _output_get_2))))
  (Class|TankGameModeBase|FreezeTank _gamemoderef)
  (Utilities|Array|Clear (Variables|/Game/_Blueprints/GameModes/BP_GameModeBase.BP_GameModeBase_C|GetRaisedFloors _gamemoderef))
  (CallFunction|SetHexagonHeight))

(event EventBeginPlay
  ;[1 1 1] Begin Play / Set Hexagons
  (bind _datatableref (CallFunction|GetCurrentLevelDataTable (Variables|Default|GetCurrentLevelNumber)))
  (Variables|Default|SetCurrentDataTableRef _datatableref)
  (bind _asbp_game_mode_base (Utilities|Casting|CastToBP_GameModeBase (Game|GetGameMode)))
  (Variables|Default|SetGameModeRef _asbp_game_mode_base)
  (CallFunction|SetHexagonHeight))

(fn ConstructionScript)

(fn GetCurrentLevelDataTable
  (params (LevelIndex :type Integer))
  (return (Utilities|Array|Get(acopy) (Variables|/Script/Engine.CompositeDataTable|GetParentTables (Variables|Default|GetCompositeDataTablesRef)) (- LevelIndex 1))))

(fn GetColumnBytesfromRow
  (params (Row :type Level%20Creation%20Structure) (Index :type Integer))
  (bind (_rowid _col1 _col2 _col3 _col4 _col5 _col6 _col7 _col8 _col9 _col10 _col11 _col12 _col13 _col14 _col15 _col16 _col17 _col18 _col19 _col20) (Utilities|Struct|BreakLevelCreation Row))
  (return (Utilities|Select :Index Index :Option%200 _col1 :Option%201 _col2 :Option%202 _col3 :Option%203 _col4 :Option%204 _col5 :Option%205 _col6 :Option%206 _col7 :Option%207 _col8 :Option%208 _col9 :Option%209 _col10 :Option%2010 _col11 :Option%2011 _col12 :Option%2012 _col13 :Option%2013 _col14 :Option%2014 _col15 :Option%2015 _col16 :Option%2016 _col17 :Option%2017 _col18 :Option%2018 _col19 :Option%2019 _col20)))

(fn MoveNextColumn
  (params (Row :type Level%20Creation%20Structure))
  (bind _amountofrows (Variables|Default|GetAmountOfRows))
  (bind _curhexrowindex (Variables|Default|GetCurHexRowIndex))
  (bind _curhexcolindex (Variables|Default|GetCurHexColIndex))
  (bind _returnvalue (* _curhexrowindex _amountofrows))
  (bind _returnvalue_2 (+ _returnvalue _curhexcolindex))
  (bind _floorhexagonref (Class|INTFloorHexagon|GetFloorHexagon(Message) (Utilities|Array|Get(acopy) (Variables|Default|GetHexagonsConst) _returnvalue_2)))
  (bind _heightbyte (CallFunction|GetColumnBytesfromRow Row (Math|Integer|%(Integer) _returnvalue_2 (Variables|Default|GetAmountOfCols))))
  (CallFunction|MoveHexagon _floorhexagonref _heightbyte _returnvalue_2)
  (Math|Integer|IncrementInt (Variables|Default|GetCurHexColIndex)
    (:%20%20
      (CallFunction|GetDataTable (Variables|Default|GetCurHexRowIndex)))))

(fn ChangetoNextRow
  (Variables|Default|SetCurHexColIndex 0)
  (Math|Integer|IncrementInt (Variables|Default|GetCurHexRowIndex)
    (:%20%20
      (if (< (Variables|Default|GetCurHexRowIndex) (Variables|Default|GetAmountOfRows))
        (return true)
        (else
          (return false))))))

(fn LoadNextLevel
  (Development|PrintString "Trying Next Level")
  (if (< (Variables|Default|GetCurrentLevelNumber) (Variables|Default|GetAmountOfLevels))
    (bind _result (Math|Integer|IncrementInt (Variables|Default|GetCurrentLevelNumber))
      (:%20%20
        (bind _datatableref (CallFunction|GetCurrentLevelDataTable _result))
        (return _datatableref)))))

(fn LoadPreviousLevel
  (Development|PrintString "Trying Previous Level")
  (if (> (Variables|Default|GetCurrentLevelNumber) 1)
    (bind _result (Math|Integer|DecrementInt (Variables|Default|GetCurrentLevelNumber))
      (:%20%20
        (bind _datatableref (CallFunction|GetCurrentLevelDataTable _result))
        (return _datatableref)))))