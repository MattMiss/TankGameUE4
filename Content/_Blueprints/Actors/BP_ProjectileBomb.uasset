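; BP_ProjectileBomb is a bomb projectile that marks its position with a decal and explodes after a short delay.
; StartBombBP moves the referenced hit decal to the mesh, shows it, prints a debug string and starts a timer that calls BlowUp.
; A detection sphere tracks whether a Player-tagged actor is in range and stores it as ActorToDamage.
; BlowUp and any damage logic are defined outside these graphs.
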(event OnComponentBeginOverlap(PlayerDetectSphere)
  (params (OverlappedComponent :type Primitive%20Component%20Object%20Reference) (OtherActor :type Actor%20Object%20Reference) (OtherComp :type Primitive%20Component%20Object%20Reference) (OtherBodyIndex :type Integer) (bFromSweep :type Boolean) (SweepResult :type Hit%20Result%20Structure%20%28by%20ref%29))
  (if (Actor|ActorHasTag OtherActor "Player")
    (Variables|Default|SetActorToDamage OtherActor)
    (Variables|Default|SetPlayerInRange true)))

(event OnComponentEndOverlap(PlayerDetectSphere)
  (params (OverlappedComponent :type Primitive%20Component%20Object%20Reference) (OtherActor :type Actor%20Object%20Reference) (OtherComp :type Primitive%20Component%20Object%20Reference) (OtherBodyIndex :type Integer))
  (if (Actor|ActorHasTag OtherActor "Player")
    (Variables|Default|SetActorToDamage OtherActor)
    (Variables|Default|SetPlayerInRange false)))

(event Custom|StartExplodeCountdown
  (Class|ProjectileBase|BlowUp))

(event EventBeginPlay)

(event Collision|EventActorBeginOverlap
  (params (OtherActor :type Actor%20Object%20Reference)))

(event EventTick
  (params (DeltaSeconds :type Float%20%28single-precision%29)))

(event EventStartBombBP
  (bind _hitdecalref (Variables|Default|GetHitDecalRef))
  (Transformation|SetActorLocation _hitdecalref (Transformation|GetWorldLocation (Variables|Default|GetProjectileMesh)) false true)
  (Rendering|SetVisibility (Variables|/Script/Engine.DecalActor|GetDecal _hitdecalref) true false)
  (Development|PrintString "Hello")
  (Utilities|Time|SetTimerbyEvent (delegate Custom|StartExplodeCountdown) 3.0))

(fn ConstructionScript)