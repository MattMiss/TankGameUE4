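; BP_FloorHexagon is a floor tile actor whose hexagon mesh raises and lowers on command.
; BeginPlay stores the start location and a raised point above it.
; StartMoving plays a raise or lower timeline that lerps the mesh from its current location, with actor tick enabled only while moving.
; On finish, the collision mesh becomes NoCollision when raised or InvisibleWall when lowered; text-label updates are left disconnected.
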(event Custom|StartMoving
  (params (Enabled :type Boolean) (HexNum :type Integer))
  ;[1 1 1] StartMoving Floor
  (Variables|Default|SetRaised Enabled)
  (Actor|Tick|SetActorTickEnabled true)
  (Variables|Default|SetCurrentLocation (Transformation|GetWorldLocation (Variables|Default|GetHexagonMesh)))
  (if (Variables|Default|GetRaised)
    (bind _height (Timeline|RaiseHexagon PlayFromStart)
      (:Update
        (Transformation|SetWorldLocation (Variables|Default|GetHexagonMesh) (Math|Vector|Lerp(Vector) (Variables|Default|GetCurrentLocation) (Variables|Default|GetRaisedLocation) _height) false false))
      (:Finished
        (Actor|Tick|SetActorTickEnabled false)
        (Collision|SetCollisionProfileName (Variables|Default|GetCollisionMesh) "NoCollision" true :!class /Script/Engine.PrimitiveComponent)))
    (else
      (bind _height_2 (Timeline|LowerHexagon PlayFromStart)
        (:Update
          (Transformation|SetWorldLocation (Variables|Default|GetHexagonMesh) (Math|Vector|Lerp(Vector) (Variables|Default|GetCurrentLocation) (Variables|Default|GetStartLocation) _height_2) false false))
        (:Finished
          (Actor|Tick|SetActorTickEnabled false)
          (Collision|SetCollisionProfileName (Variables|Default|GetCollisionMesh) "InvisibleWall" true :!class /Script/Engine.PrimitiveComponent))))))

(event EventBeginPlay
  (bind _hexagonmesh (Variables|Default|GetHexagonMesh))
  (bind _returnvalue (Transformation|GetWorldLocation _hexagonmesh))
  ;[1 1 1] Begin Play / Set Hexagon World Location
  (Variables|Default|SetStartLocation _returnvalue)
  (Variables|Default|SetRaisedLocation (+ _returnvalue "0, 0,500.000000")))

(fn ConstructionScript)

(fn GetFloorHexagon
  (return self))